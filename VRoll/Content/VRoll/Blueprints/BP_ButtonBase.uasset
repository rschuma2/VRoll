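; BP_ButtonBase is a physically pressable VR button base with configurable label text and an empty ButtonAction function.
; When a motion controller's GrabSphere enters the Box, a gated Tick moves the Cube with the sphere along local Z, clamped to PressDistance.
; Reaching near full depth calls ButtonAction and resets; leaving the box also resets.
; Reset closes the gate and eases the Cube back with a timeline before re-arming.
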(event `self.ReceiveTick`
  (params (DeltaSeconds :type "Float (single-precision)"))
  (bind (_buttonstartlocation_x _buttonstartlocation_y _buttonstartlocation_z) (`KismetMathLibrary.BreakVector` (`self.ButtonStartLocation`)))
  (bind _buttonstartlocation (`self.ButtonStartLocation`))
  (bind _z (.z _buttonstartlocation))
  (bind (_relativelocation_x _relativelocation_y _relativelocation_z) (`KismetMathLibrary.BreakVector` (`SceneComponent.RelativeLocation` (`self.Cube`))))
  (bind (_returnvalue_x _returnvalue_y _returnvalue_z) (`KismetMathLibrary.BreakVector` (- (`KismetMathLibrary.InverseTransformLocation` (`self.GetTransform`) (`SceneComponent.K2_GetComponentLocation` (`self.GrabSphereRef`))) (`self.ButtonStartLocation`))))
  (bind (_returnvalue_x_2 _returnvalue_y_2 _returnvalue_z_2) (`KismetMathLibrary.BreakVector` (+ _buttonstartlocation (`KismetMathLibrary.MakeVector` 0.0 0.0 _returnvalue_z))))
  (`/Engine/EditorBlueprintResources/StandardMacros.Gate` true :!label _label
    (:`Exit`
      (`SceneComponent.K2_SetRelativeLocation` (`self.Cube`) (`KismetMathLibrary.MakeVector` _returnvalue_x_2 _returnvalue_y_2 (`KismetMathLibrary.FClamp` _returnvalue_z_2 (- _z (`self.PressDistance`)) _z)) false false)
      (if (`KismetMathLibrary.NearlyEqual_FloatFloat` _relativelocation_z (- _buttonstartlocation_z (`self.PressDistance`)) 2.5)
        (`self.ButtonAction`)
        (`self.ResetButton`)))))

(event `self.Box.OnComponentBeginOverlap`
  (params (OverlappedComponent :type "PrimitiveComponent Object Reference") (OtherActor :type "Actor Object Reference") (OtherComp :type "PrimitiveComponent Object Reference") (OtherBodyIndex :type Integer) (bFromSweep :type Boolean) (SweepResult :type "HitResult Structure (by ref)"))
  (if (not (`self.ButtonPressed`))
    (bind _asbp_motion_controller (cast `/Game/VirtualRealityBP/Blueprints/BP_MotionController` OtherActor))
    (bind _grabsphere (`/Game/VirtualRealityBP/Blueprints/BP_MotionController.GrabSphere` _asbp_motion_controller))
    (if (== _grabsphere OtherComp)
      (set `self.ButtonPressed` true)
      (set `self.GrabSphereRef` _grabsphere)
      (set `self.ButtonStartLocation` (`SceneComponent.RelativeLocation` (`self.Cube`)))
      (goto _label :!via `Open`))))

(event `self.Box.OnComponentEndOverlap`
  (params (OverlappedComponent :type "PrimitiveComponent Object Reference") (OtherActor :type "Actor Object Reference") (OtherComp :type "PrimitiveComponent Object Reference") (OtherBodyIndex :type Integer))
  (bind _asbp_motion_controller (cast `/Game/VirtualRealityBP/Blueprints/BP_MotionController` OtherActor))
  (if (== (`/Game/VirtualRealityBP/Blueprints/BP_MotionController.GrabSphere` _asbp_motion_controller) OtherComp)
    (`self.ResetButton`)))

(event `ResetButton`
  (bind (_buttonstartlocation_x _buttonstartlocation_y _buttonstartlocation_z) (`KismetMathLibrary.BreakVector` (`self.ButtonStartLocation`)))
  (bind (_relativelocation_x _relativelocation_y _relativelocation_z) (`KismetMathLibrary.BreakVector` (`SceneComponent.RelativeLocation` (`self.Cube`))))
  (`|ExecutionSequence`
    (:`then_0`
      (goto _label :!via `Close`))
    (:`then_1`
      (bind (_direction _driver) (`Timeline|SnapBackTimeline` :!via `PlayFromStart`)
        (:`Update`
          (`SceneComponent.K2_SetRelativeLocation` (`self.Cube`) (`KismetMathLibrary.MakeVector` _buttonstartlocation_x _buttonstartlocation_y (`KismetMathLibrary.Lerp` _relativelocation_z _buttonstartlocation_z _driver)) false false))
        (:`Finished`
          (set `self.ButtonPressed` false))))))

(fn `ButtonAction`)

(fn `UserConstructionScript`
  (`TextRenderComponent.K2_SetText` (`self.TextRender`) (`self.ButtonText`)))